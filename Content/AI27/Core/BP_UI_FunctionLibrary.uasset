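; Blueprint function library of UI lookup helpers for the AIS Simulator.
; GetOverallUI casts the game state to BP_AIS_Simulator_GameState and returns its OverallUI, printing a message when the cast fails or the reference is invalid.
; GetAppPlatformWidget searches all widgets, not just top-level ones, for WBP_AiS_AppPlatform and returns the first if valid.
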(fn GetOverallUI
  (bind _asbp_ais_simulator_game_state (Utilities|Casting|CastToBP_AIS_Simulator_GameState (Game|GetGameState))
    (:then
      (bind _overallui (Variables|/Game/AI27/Core/BP_AIS_Simulator_GameState.BP_AIS_Simulator_GameState_C|GetOverallUI _asbp_ais_simulator_game_state)
        (:then
          _)
        (:else
          (Development|PrintString 0 "Error: OverallUI is not valid, check the variable in the game state, make shure to call this after the overall has been created.")))
      (return _overallui))
    (:CastFailed
      (Development|PrintString 0 "Warning: AIS Simulaotr GameState not found."))))

(fn GetAppPlatformWidget
  (bind _foundwidgets (Widget|GetAllWidgetsOfClass 0 "/Game/AI27/UI/AiSApp/WBP_AiS_AppPlatform.WBP_AiS_AppPlatform_C" false))
  (Utilities|IsValid (Utilities|Array|Get(acopy) _foundwidgets)
    (:Is%20Valid
      (return (Utilities|Array|Get(acopy) _foundwidgets)))
    (:Is%20Not%20Valid
      (return 0))))